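; Pressure plate actor that sinks when something enters its box trigger and rises again once nothing is overlapping it.
; Box begin and end overlaps check the actor's overlap count, so only the first arrival and last departure toggle the Overlapped flag.
; The PressurePlatePosition timeline plays or reverses to lerp the static mesh's relative location slightly downward and back.
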(event OnComponentBeginOverlap(Box)
  (params (OverlappedComponent :type Primitive%20Component%20Object%20Reference) (OtherActor :type Actor%20Object%20Reference) (OtherComp :type Primitive%20Component%20Object%20Reference) (OtherBodyIndex :type Integer) (bFromSweep :type Boolean) (SweepResult :type Hit%20Result%20Structure%20%28by%20ref%29))
  (switch int (Utilities|Array|Length (Collision|GetOverlappingActors 0 :!class /Script/Engine.Actor))
    (:1
      (Variables|Default|SetOverlapped true)
      (bind _float (Timeline|PressurePlatePosition Play)
        (:Update
          (Transformation|SetRelativeLocation (Variables|Default|GetStaticMesh) (Math|Vector|Lerp(Vector) "0, 0, 0" "0, 0,-10.000000" _float) false false))))))

(event OnComponentEndOverlap(Box)
  (params (OverlappedComponent :type Primitive%20Component%20Object%20Reference) (OtherActor :type Actor%20Object%20Reference) (OtherComp :type Primitive%20Component%20Object%20Reference) (OtherBodyIndex :type Integer))
  (if (not (Math|Conversions|ToBoolean(Integer) (Utilities|Array|Length (Collision|GetOverlappingActors 0 :!class /Script/Engine.Actor))))
    (Variables|Default|SetOverlapped false)
    (bind _float (Timeline|PressurePlatePosition Reverse)
      (:Update
        (Transformation|SetRelativeLocation (Variables|Default|GetStaticMesh) (Math|Vector|Lerp(Vector) "0, 0, 0" "0, 0,-10.000000" _float) false false)))))

(event EventBeginPlay)

(event Collision|EventActorBeginOverlap
  (params (OtherActor :type Actor%20Object%20Reference)))

(event EventTick
  (params (DeltaSeconds :type Float%20%28single-precision%29)))

(fn ConstructionScript)